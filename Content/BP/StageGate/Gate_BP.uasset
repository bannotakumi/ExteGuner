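; Gate_BP is a stage gate that loses HP when enemies hit it.
; On BeginPlay it takes its starting HP from the MaxHP of its GateHPbar widget, then copies the current HP into that widget every Tick.
; When an AI_Enemy begins overlapping AttackCollisionBox, ReciveDamage subtracts that enemy's ATK from GateHP.
; The file contains no clamping or destruction logic for when HP runs out.
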(event `self.ReceiveBeginPlay`
  ;[1 1 1] ゲートのHPの初期化
  (bind _asgate_hpbar (cast `/Game/BP/Widget/GateHPbar` (`WidgetComponent.GetWidget` (`self.GateHPbar`))))
  (set `self.GateHP` (`/Game/BP/Widget/GateHPbar.MaxHP` _asgate_hpbar)))

(event `self.ReceiveTick`
  (params (DeltaSeconds :type "Float (single-precision)"))
  ;[1 1 1] ゲートのＨＰの更新
  (bind _asgate_hpbar (cast `/Game/BP/Widget/GateHPbar` (`WidgetComponent.GetWidget` (`self.GateHPbar`))))
  (set `/Game/BP/Widget/GateHPbar.HP` (`self.GateHP`) _asgate_hpbar))

(event `self.AttackCollisionBox.OnComponentBeginOverlap`
  (params (OverlappedComponent :type "PrimitiveComponent Object Reference") (OtherActor :type "Actor Object Reference") (OtherComp :type "PrimitiveComponent Object Reference") (OtherBodyIndex :type Integer) (bFromSweep :type Boolean) (SweepResult :type "HitResult Structure (by ref)"))
  ;[1 1 1] 敵からのダメージ処理
  (bind _asai_enemy (cast `/Game/BP/Enemy/AI_Enemy` OtherActor))
  (`self.ReciveDamage` (`/Game/BP/Enemy/AI_Enemy.ATK` _asai_enemy)))

(fn `ReciveDamage`
  (params (EnemyATK :type "Float (double-precision)"))
  (set `self.GateHP` (- (`self.GateHP`) EnemyATK)))

(fn `UserConstructionScript`)