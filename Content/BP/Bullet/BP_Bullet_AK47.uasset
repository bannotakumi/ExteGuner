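; AK47 bullet actor that loads speed, damage and type from the AK47_Status data table row matching the game mode's AK47 rank.
; A Rotation event sets its velocity and facing; Tick sweeps it forward and destroys it after DeleteTime.
; Box overlaps only spawn a hit particle, with the enemy cast left disconnected.
; Getters and DestroyBullet expose damage, type and removal to other objects.
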(event `self.ReceiveBeginPlay`
  (`self.BeginDataSetting`))

(event `self.ReceiveActorBeginOverlap`
  (params (OtherActor :type "Actor Object Reference")))

(event `self.ReceiveTick`
  (params (DeltaSeconds :type "Float (single-precision)"))
  (bind _boxcol (`self.BoxCol`))
  (`self.K2_SetActorLocationAndRotation` (+ (`self.K2_GetActorLocation`) (`self.World_Vec`)) (struct) true)
  (`/Engine/EditorBlueprintResources/StandardMacros.IsValid` _boxcol
    (:`Is Valid`
      (`SceneComponent.K2_SetWorldRotation` _boxcol (`self.PickGun_Rotation`) false false)
      (bind _output_get (set `self.deleteCountTimer` (+ DeltaSeconds (`self.deleteCountTimer`))))
      (if (> _output_get (`self.deleteTime`))
        (`self.K2_DestroyActor`)))))

(event `/Game/BP/Interface/I_BP_Bullet.Rotation`
  (params (Bullet_Rot :type "Rotator Structure"))
  (bind _returnvalue (`KismetMathLibrary.ComposeRotators` (struct :`Yaw` 90.0) Bullet_Rot))
  (set `self.World_Vec` (* (`KismetMathLibrary.GreaterGreater_VectorRotator` (`self.World_Vec`) _returnvalue) (`self.Speed`)))
  (set `self.PickGun_Rotation` _returnvalue))

(event `self.BoxCol.OnComponentBeginOverlap`
  (params (OverlappedComponent :type "PrimitiveComponent Object Reference") (OtherActor :type "Actor Object Reference") (OtherComp :type "PrimitiveComponent Object Reference") (OtherBodyIndex :type Integer) (bFromSweep :type Boolean) (SweepResult :type "HitResult Structure (by ref)"))
  (`GameplayStatics.SpawnEmitterAtLocation` "/Game/Resources/GunEffects/P_ky_hit2.P_ky_hit2" (`self.K2_GetActorLocation` self)))

(fn `BeginDataSetting`
  (bind _asstage_game_mode (cast `/Game/BP/GameMode/StageGameMode` (`GameplayStatics.GetGameMode`)))
  (bind _returnvalue (`|GetDataTableRow` "/Game/Resources/GunDataTableCSV/AK47_Status.AK47_Status" (`KismetStringLibrary.Conv_StringToName` (`KismetStringLibrary.Conv_IntToString` (`/Game/BP/GameMode/StageGameMode.Rank_AK47` _asstage_game_mode))))
    (:`then`
      (set `self.Speed` (`.Speed_49_06E0B5A44B11587ADDCC25B2C3214F1A` (break `/Game/BP/Structure/GunDataTable` _returnvalue)))
      (set `self.bulletDamage` (`.BulletDamage_50_5E5BAAE64D9E6BB9BA0F639DE38EE0A8` (break `/Game/BP/Structure/GunDataTable` _returnvalue)))
      (set `self.BulletType` (`.BulletType_51_2B6CC9D149000D23E680E4852D8B8370` (break `/Game/BP/Structure/GunDataTable` _returnvalue))))))

(fn `DestroyBullet`
  (`self.K2_DestroyActor`)
  (return))

(fn `GetBulletType`
  (returns (BulletType :type Name))
  (return (`self.BulletType`)))

(fn `GetDamage`
  (returns (damage :type Integer))
  (return (`self.bulletDamage`)))

(fn `UserConstructionScript`)