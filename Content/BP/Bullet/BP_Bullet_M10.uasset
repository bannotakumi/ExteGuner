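; BP_Bullet_M10 is a projectile actor, apparently for an M10 weapon, that flies straight and sparks on enemies.
; Its Rotation event turns a supplied rotator into a speed-scaled movement vector and a collision box rotation.
; Tick applies that vector as a swept per-frame offset, without delta-time scaling, and re-applies the box rotation.
; Overlapping an AI_Enemy only spawns a hit emitter; damage and destruction are exposed as functions.
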(event `self.ReceiveBeginPlay`)

(event `self.ReceiveActorBeginOverlap`
  (params (OtherActor :type "Actor Object Reference")))

(event `self.ReceiveTick`
  (params (DeltaSeconds :type "Float (single-precision)"))
  (bind _boxcol (`self.BoxCol`))
  (`self.K2_SetActorLocationAndRotation` (+ (`self.K2_GetActorLocation`) (`self.World_Vec`)) (struct) true)
  (`/Engine/EditorBlueprintResources/StandardMacros.IsValid` _boxcol
    (:`Is Valid`
      (`SceneComponent.K2_SetWorldRotation` _boxcol (`self.PickGun_Rotation`) false false))))

(event `/Game/BP/Interface/I_BP_Bullet.Rotation`
  (params (Bullet_Rot :type "Rotator Structure"))
  (bind _returnvalue (`KismetMathLibrary.ComposeRotators` (struct :`Yaw` 90.0) Bullet_Rot))
  (set `self.World_Vec` (* (`KismetMathLibrary.GreaterGreater_VectorRotator` (`self.World_Vec`) _returnvalue) (`self.Speed`)))
  (set `self.PickGun_Rotation` _returnvalue))

(event `self.BoxCol.OnComponentBeginOverlap`
  (params (OverlappedComponent :type "PrimitiveComponent Object Reference") (OtherActor :type "Actor Object Reference") (OtherComp :type "PrimitiveComponent Object Reference") (OtherBodyIndex :type Integer) (bFromSweep :type Boolean) (SweepResult :type "HitResult Structure (by ref)"))
  (cast `/Game/BP/Enemy/AI_Enemy` OtherActor)
  (`GameplayStatics.SpawnEmitterAtLocation` "/Game/Resources/GunEffects/P_ky_hit2.P_ky_hit2" (`self.K2_GetActorLocation` self)))

(fn `DestroyBullet`
  (`self.K2_DestroyActor`)
  (return))

(fn `GetDamage`
  (returns (damage :type Integer))
  (return (`self.bulletDamage`)))

(fn `UserConstructionScript`)