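; Coin item Actor that spins, blinks, then automatically adds its Money value to the player's funds when its lifetime ends.
; All logic runs on Tick, rotating its meshes and accumulating a timer that toggles their visibility at intervals after a short delay.
; On expiry it spawns an emitter, increases HaveMoney on StageGameMode and destroys itself, with no pickup or overlap check.
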(event `self.ReceiveTick`
  (params (DeltaSeconds :type "Float (single-precision)"))
  (bind _time (`self.Time`))
  ;[1 1 1] 敵回転処理
  (`SceneComponent.K2_AddLocalRotation` (`self.Item`) (`KismetMathLibrary.MakeRotator` 0.0 0.0 (+ (`self.Rotate`) DeltaSeconds)) false false)
  (`SceneComponent.K2_AddLocalRotation` (`self.StaticMesh1`) (`KismetMathLibrary.MakeRotator` 0.0 0.0 (+ (`self.Rotate`) DeltaSeconds)) false false)
  (`SceneComponent.K2_AddLocalRotation` (`self.StaticMesh`) (`KismetMathLibrary.MakeRotator` 0.0 0.0 (+ (`self.Rotate`) DeltaSeconds)) false false)
  (set `self.Time` (+ (`self.Time`) DeltaSeconds))
  (if (> _time 2.0)
    (`SceneComponent.SetVisibility` (`self.Item`) (>= (mod (/ (- _time 2.0) 0.5) 2.0) 0.5) false)
    (`SceneComponent.SetVisibility` (`self.StaticMesh`) (>= (mod (/ (- _time 2.0) 0.5) 2.0) 0.5) false)
    (`SceneComponent.SetVisibility` (`self.StaticMesh1`) (>= (mod (/ (- _time 2.0) 0.5) 2.0) 0.5) false)
    ;[1 1 1] 敵消滅処理
    (if (> (`self.Time`) 5.0)
      ;[1 1 1] effect処理
      (`GameplayStatics.SpawnEmitterAtLocation` null (`SceneComponent.K2_GetComponentLocation` (`self.Item`)))
      ;[1 1 1] お金の処理
      (bind _asstage_game_mode (cast `/Game/BP/GameMode/StageGameMode` (`GameplayStatics.GetGameMode`)))
      (set `/Game/BP/GameMode/StageGameMode.haveMoney` (+ (`/Game/BP/GameMode/StageGameMode.haveMoney` _asstage_game_mode) (`self.Money`)) _asstage_game_mode)
      (`self.K2_DestroyActor`))))

(fn `UserConstructionScript`)