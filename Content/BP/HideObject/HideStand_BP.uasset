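; HideStand_BP is an actor in the HideObject folder, apparently a hiding spot that carries a teleport destination.
; Every Tick it turns on custom depth rendering for its static mesh, with no condition.
; Its functions return the actor's location and read or set a stored teleport vector; the actor itself performs no teleport.
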(event `self.ReceiveTick`
  (params (DeltaSeconds :type "Float (single-precision)"))
  (`PrimitiveComponent.SetRenderCustomDepth` (`self.StaticMeshComponent`) true))

(fn `GetSelfLocation`
  (returns (SelfLocation :type "Vector Structure"))
  (return (`self.K2_GetActorLocation`)))

(fn `GetTeleportLocation`
  (returns (TeleportLocation :type "Vector Structure"))
  (return (`self.Teleport_Vector`)))

(fn `SetTeleportVec`
  (params (teleportVec :type "Vector Structure"))
  (set `self.Teleport_Vector` teleportVec)
  (return))

(fn `UserConstructionScript`)