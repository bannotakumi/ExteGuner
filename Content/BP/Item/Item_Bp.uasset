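; Item actor that spins, blinks as a warning and then removes itself after a short lifetime.
; Tick adds a yaw step to the Item component, computed as Rotate plus DeltaSeconds rather than scaled by it, so spin speed depends on frame rate.
; Tick also accumulates Time, which after a delay toggles visibility through a modulo test and finally destroys the actor.
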(event `self.ReceiveTick`
  (params (DeltaSeconds :type "Float (single-precision)"))
  (bind _time (`self.Time`))
  ;[1 1 1] 敵回転処理
  (`SceneComponent.K2_AddLocalRotation` (`self.Item`) (`KismetMathLibrary.MakeRotator` 0.0 0.0 (+ (`self.Rotate`) DeltaSeconds)) false false)
  (set `self.Time` (+ (`self.Time`) DeltaSeconds))
  (if (> _time 2.0)
    (`SceneComponent.SetVisibility` (`self.Item`) (>= (mod (/ (- _time 2.0) 0.5) 2.0) 0.5) false)
    ;[1 1 1] 敵消滅処理
    (if (> (`self.Time`) 5.0)
      (`self.K2_DestroyActor`))))

(fn `UserConstructionScript`)