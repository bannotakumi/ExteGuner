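; VR AK47 pickup that attaches to hand sockets, fires automatically while used, and has a detachable magazine.
; Tick spawns bullets and muzzle flash on a timer, syncing ammo and per-hand rumble flags to StageGameMode.
; A dropped gun hitting Ground or falling below the floor limit reattaches to HiddenPlayerBody.
; Stats reload every Tick from M4A1_Status by RankM4A1, and Use plays the M4A1 sound, despite the AK47 identity.
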(event `self.ReceiveBeginPlay`
  (bind _asstage_game_mode (cast `/Game/BP/GameMode/StageGameMode` (`GameplayStatics.GetGameMode`)))
  (set `self.Bullets` (`/Game/BP/GameMode/StageGameMode.remBullets_AK47` _asstage_game_mode)))

(event `self.ReceiveTick`
  (params (DeltaSeconds :type "Float (single-precision)"))
  (bind _usesound (`self.UseSound`))
  (bind _returnvalue (`SceneComponent.GetSocketTransform` (`self.SkeletalMeshComponent`) "b_gun_muzzleflash" "RTS_World"))
  (bind (_returnvalue_x _returnvalue_y _returnvalue_z) (`KismetMathLibrary.BreakVector` (`SceneComponent.K2_GetComponentLocation` (`self.SkeletalMeshComponent`))))
  ;[1 1 1] Update
  ;;[1 1 1] 地面より下に落ちた場合テレポートで戻る
  (bind _asstage_game_mode (cast `/Game/BP/GameMode/StageGameMode` (`GameplayStatics.GetGameMode`)))
  (if (> (`/Game/BP/GameMode/StageGameMode.stageLimitFloor` _asstage_game_mode) _returnvalue_z)
    (set `self.teleportCheck` true))
  (`self.BeginDataSetting`)
  ;;[1 1 1] マガジンの有無に合わせてメッシュを切り替える
  (if (`self.magazineChack`)
    (`SceneComponent.SetVisibility` (`self.SkeletalMeshComponent`) true false)
    (`SceneComponent.SetVisibility` (`self.NoMagazine`) false false)
    (else
      (`SceneComponent.SetVisibility` (`self.SkeletalMeshComponent`) false false)
      (`SceneComponent.SetVisibility` (`self.NoMagazine`) true false)))
  ;;[1 1 1] レーザーポインターの可視化
  (set `WidgetInteractionComponent.bShowDebug` (`self.laserShowDebug`) (`self.WidgetInteraction`))
  (if (`self.teleportCheck`)
    ;;[1 1 1] 位置を常にHMDに合わせる
    ;;;[1 1 1] 銃の回転
    (`self.K2_SetActorRotation` (`self.addGunSetRot`))
    ;;;[1 1 1] 位置をワールドからローカルに変更
    (`self.K2_SetActorLocation` (`self.addGunSetTrans`))
    ;;;[1 1 1] HiddenPlayerBodyへ親子付け
    (`self.K2_AttachToActor` self (`self.HiddenPlayerBody`) "None" "KeepRelative" "KeepRelative" "KeepRelative" true)
    (set `self.teleportCheck` false)
    (`PrimitiveComponent.SetSimulatePhysics` (`self.SkeletalMeshComponent`) false))
  (bind _output_get (set `self.bulletTimeCounter` (- (`self.bulletTimeCounter`) DeltaSeconds)))
  ;;[1 1 1] マガジンの残弾チェック
  (bind _bulletchack (`self.Magazine_Check`))
  (if _bulletchack
    (set `self.Gun_Rotation` (`self.K2_GetActorRotation`))
    ;;[1 1 1] 銃を連射中か否か
    (if (`self.BulletShotCheck`)
      ;;[1 1 1] 銃の連射感覚タイマー
      (if (> 0.0 _output_get)
        ;;[1 1 1] タイマー初期化
        (set `self.bulletTimeCounter` (`self.iniBulletTimer`))
        ;;[1 1 1] 弾発射
        ;;;[1 1 1] 弾の指定
        (bind _returnvalue_2 (`|SpawnActorFromClass` "/Game/BP/Bullet/BP_Bullet_AK47.BP_Bullet_AK47_C" _returnvalue "Undefined" "OverrideRootScale" null null))
        (`self.ShotBullet` _returnvalue_2)
        (bind _output_get_2 (set `self.SocketTransform` _returnvalue))
        ;;;[1 1 1] 発射時のエフェクト指定
        (`NiagaraFunctionLibrary.SpawnSystemAtLocation` "/Game/Resources/effect/FX/N_MuzzleFlash.N_MuzzleFlash" (.location _output_get_2) (`KismetMathLibrary.ComposeRotators` (struct :`Yaw` 180.0) (`self.Gun_Rotation`)))
        ;;[1 1 1] 残弾を減らす
        (bind _output_get_3 (set `self.Bullets` (- (`self.Bullets`) 1)))
        (bind _asstage_game_mode_2 (cast `/Game/BP/GameMode/StageGameMode` (`GameplayStatics.GetGameMode`)))
        (set `/Game/BP/GameMode/StageGameMode.remBullets_AK47` _output_get_3 _asstage_game_mode_2)
        (bind _asstage_game_mode_3 (cast `/Game/BP/GameMode/StageGameMode` (`GameplayStatics.GetGameMode`)))
        (if (`|EnumEquality` (`self.hand`) "Left")
          (set `/Game/BP/GameMode/StageGameMode.ranbleFlagLeft` true _asstage_game_mode_3)
          (else
            (set `/Game/BP/GameMode/StageGameMode.ranbleFlagRight` true _asstage_game_mode_3)))))
    (else
      ;;[1 1 1] 残弾が切れたら音も消す
      (`/Engine/EditorBlueprintResources/StandardMacros.IsValid` _usesound
        (:`Is Valid`
          (`AudioComponent.Stop` _usesound)
          (`GameplayStatics.SpawnSoundAtLocation` "/Game/Resources/SE/AirShot.AirShot" (`self.K2_GetActorLocation`) (struct) 1.0 1.0 0.0 null null)
          (set `self.UseSound` null)
          (set `self.BulletShotCheck` false)
          (bind _asstage_game_mode_4 (cast `/Game/BP/GameMode/StageGameMode` (`GameplayStatics.GetGameMode`)))
          (set `/Game/BP/GameMode/StageGameMode.ranbleFlagLeft` false _asstage_game_mode_4)
          (set `/Game/BP/GameMode/StageGameMode.ranbleFlagRight` false _asstage_game_mode_4))))))

(event `/Game/VirtualRealityBP/Blueprints/PickupActorInterface.Pickup`
  (params (AttachTo :type "SceneComponent Object Reference") (SocketName :type Name))
  (bind _rootcomponent (`self.RootComponent`))
  (bind _skeletalmeshcomponent (`self.SkeletalMeshComponent`))
  ;[1 1 1] 持った時の音指定
  (`GameplayStatics.SpawnSoundAtLocation` "/Game/Resources/GunSounds/sw_Wep_AR_Equip.sw_Wep_AR_Equip" (`self.K2_GetActorLocation`) (struct) 1.0 1.0 0.0 null null)
  (`PrimitiveComponent.SetSimulatePhysics` _skeletalmeshcomponent false)
  (if (== SocketName "Right")
    (`SceneComponent.K2_AttachToComponent` _rootcomponent AttachTo "Ak_Socket_Right" "KeepWorld" "KeepWorld" "KeepWorld" false)
    (else
      (`SceneComponent.K2_AttachToComponent` _rootcomponent AttachTo "Ak_Socket_Left" "KeepWorld" "KeepWorld" "KeepWorld" false)))
  (`SceneComponent.K2_SetRelativeLocationAndRotation` :`self` _skeletalmeshcomponent :`NewLocation` (0.0 -2.0 -1.0))
  (set `self.teleportCheck` false))

(event `/Game/VirtualRealityBP/Blueprints/PickupActorInterface.Drop`
  (`PrimitiveComponent.SetSimulatePhysics` (`self.SkeletalMeshComponent`) true)
  (`self.K2_DetachFromActor` "KeepWorld" "KeepWorld" "KeepWorld"))

(event `/Game/VirtualRealityBP/Blueprints/PickupActorInterface.UnUse`
  (bind _usesound (`self.UseSound`))
  ;[1 1 1] 銃を撃っていない状態
  (`/Engine/EditorBlueprintResources/StandardMacros.IsValid` _usesound
    (:`Is Valid`
      (`AudioComponent.Stop` _usesound)
      (set `self.BulletShotCheck` false)
      (bind _asstage_game_mode (cast `/Game/BP/GameMode/StageGameMode` (`GameplayStatics.GetGameMode`)))
      (set `/Game/BP/GameMode/StageGameMode.ranbleFlagLeft` false _asstage_game_mode)
      (set `/Game/BP/GameMode/StageGameMode.ranbleFlagRight` false _asstage_game_mode))))

(event `/Game/VirtualRealityBP/Blueprints/PickupActorInterface.Detach`
  ;[1 1 1] 手放す
  (`self.K2_DetachFromActor` "KeepWorld" "KeepWorld" "KeepWorld"))

(event `self.AddMagazine`
  ;[1 1 1] マガジンの追加
  (if (not (`self.magazineChack`))
    (set `self.Bullets` (`self.maxBullets`))
    ;;[1 1 1] マガジン装着時のSE
    ;;;[1 1 1] リロード音指定
    (`GameplayStatics.SpawnSoundAtLocation` "/Game/Resources/GunSounds/MagazineSet.MagazineSet" (`self.K2_GetActorLocation`) (struct) 1.0 1.0 0.0 null null false)
    (set `self.magazineChack` true)))

(event `self.DropMagazine`
  ;[1 1 1] マガジンを落とす
  (if (`self.magazineChack`)
    (set `self.Bullets` 0)
    ;;[1 1 1] マガジンドロップ時のSE
    ;;;[1 1 1] マガジンを落とした時の音指定
    (`GameplayStatics.SpawnSoundAtLocation` "/Game/Resources/GunSounds/MagazineDelete.MagazineDelete" (`self.K2_GetActorLocation`) (struct) 1.0 1.0 0.0 null null false)
    ;;[1 1 1] マガジンの生成
    ;;;[1 1 1] 生成するマガジンを指定
    (`|SpawnActorFromClass` "/Game/BP/Magazine/MagazineEmpty_AK47.MagazineEmpty_AK47_C" (`SceneComponent.GetSocketTransform` (`self.SkeletalMeshComponent`) "b_rifleMag" "RTS_World") "Undefined" "OverrideRootScale" null null)
    (set `self.magazineChack` false)))

(event `self.SkeletalMeshComponent.OnComponentHit`
  (params (HitComponent :type "PrimitiveComponent Object Reference") (OtherActor :type "Actor Object Reference") (OtherComp :type "PrimitiveComponent Object Reference") (NormalImpulse :type "Vector Structure") (Hit :type "HitResult Structure (by ref)"))
  ;[1 1 1] 地面に落ちたら自分を所定の位置に戻す
  ;;[1 1 1] 地面(TagがGround)に当たったら
  ;;;[1 1 1] オブジェクトのnullチェック
  (if (`KismetSystemLibrary.IsValid` OtherActor)
    (if (`self.ActorHasTag` OtherActor "Ground")
      (set `self.teleportCheck` true))))

(event `self.ElectrostaticTrigger`
  (params (triggerTouth :type Boolean))
  ;[1 1 1] 静電容量トリガーに触れたとき
  (set `self.laserShowDebug` triggerTouth))

(fn `BeginDataSetting`
  (bind _asstage_game_mode (cast `/Game/BP/GameMode/StageGameMode` (`GameplayStatics.GetGameMode`)))
  (bind _returnvalue (`|GetDataTableRow` "/Game/Resources/GunDataTableCSV/M4A1_Status.M4A1_Status" (`KismetStringLibrary.Conv_StringToName` (`KismetStringLibrary.Conv_IntToString` (`/Game/BP/GameMode/StageGameMode.Rank_M4A1` _asstage_game_mode))))
    (:`then`
      (set `self.maxBullets` (break `/Game/BP/Structure/GunDataTable` _returnvalue))
      (set `self.iniBulletTimer` (`.BulletTimer_35_71F9300848D0835182E38A984F41E7F7` (break `/Game/BP/Structure/GunDataTable` _returnvalue)))
      (set `self.addGunSetTrans` (`KismetMathLibrary.MakeVector` (`.AddGunSetTransX_37_C961513346778771816CE2A4307B5AB8` (break `/Game/BP/Structure/GunDataTable` _returnvalue)) (`.AddGunSetTransY_38_D33E52934DED0A455BFB58BB3BF9D3C5` (break `/Game/BP/Structure/GunDataTable` _returnvalue)) (`.AddGunSetTransZ_39_13B0496D4AD8D42881954D83BA59A83F` (break `/Game/BP/Structure/GunDataTable` _returnvalue))))
      (set `self.addGunSetRot` (`KismetMathLibrary.MakeRotator` (`.AddGunSetRotX_40_4DD348D74D82AB63C5E1AE83FCA83C7A` (break `/Game/BP/Structure/GunDataTable` _returnvalue)) (`.AddGunSetRotY_41_6CD517BF428E07C7CDC4449D9A0372B3` (break `/Game/BP/Structure/GunDataTable` _returnvalue)) (`.AddGunSetRotZ_42_B52D1FE94C7D70ECA8B1FE8D9B887C21` (break `/Game/BP/Structure/GunDataTable` _returnvalue))))
      (bind _asstage_game_mode_2 (cast `/Game/BP/GameMode/StageGameMode` (`GameplayStatics.GetGameMode`)))
      (set `/Game/BP/GameMode/StageGameMode.rankUpPrice_AK47` (`.RankUpPrice_55_1CBF87014823F9801FD425A7081ED586` (break `/Game/BP/Structure/GunDataTable` _returnvalue)) _asstage_game_mode_2))))

(fn `Get_PickGun_Rotation`
  (returns (PickGun_Rot :type "Rotator Structure"))
  (return (`self.Gun_Rotation`)))

(fn `GetBulletType`
  (returns (damageType :type Name))
  (return "Normal"))

(fn `GetDamage`
  (returns (damage :type Integer))
  (return 1))

(fn `GetGunTag`
  (returns (tagName :type Name))
  (return "AK47"))

(fn `GetHandGuardSocket`
  (returns (SocketLocation :type "Vector Structure"))
  (return (`SceneComponent.K2_GetComponentLocation` (`self.HandGuardSocket`))))

(fn `InMagCheck`
  (returns (magazineCheck :type Boolean))
  (return (`self.magazineChack`)))

(fn `Magazine_Check`
  (returns (BulletChack :type Boolean))
  ;[1 1 1] 残弾があればtrue,なければfalse
  (return (> (`self.Bullets`) 0)))

(fn `ShotBullet`
  (params (Bullet :type "/Game/BP/Interface/I_BP_Bullet Interface"))
  (`/Game/BP/Interface/I_BP_Bullet.Rotation` Bullet (`self.Gun_Rotation`)))

(fn `Use`
  (params (hand :type "EControllerHand Enum" :default "Left"))
  (bind _returnvalue (`self.K2_GetActorLocation`))
  ;[1 1 1] 銃声
  (set `self.hand` hand)
  (bind _bulletchack (`self.Magazine_Check`))
  (if _bulletchack
    ;;[1 1 1] 撃った時の音
    (bind _returnvalue_2 (`GameplayStatics.SpawnSoundAtLocation` "/Game/Resources/GunSounds/M4A1.M4A1" _returnvalue (struct) 1.0 1.0 0.0 null null false))
    (set `self.UseSound` _returnvalue_2)
    (set `self.BulletShotCheck` true)
    (else
      ;[1 1 1] 空撃ちの音
      (`GameplayStatics.SpawnSoundAtLocation` "/Game/Resources/SE/AirShot.AirShot" _returnvalue (struct) 1.0 1.0 0.0 null null false)))
  (return))

(fn `UserConstructionScript`)